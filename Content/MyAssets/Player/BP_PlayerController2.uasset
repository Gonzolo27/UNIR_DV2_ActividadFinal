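; BP_PlayerController2 is a player controller that routes player input to the controlled BP_Character_2 pawn.
; Axis inputs drive movement along the character's forward and right vectors, plus camera pitch and yaw.
; Action presses call the character's physical Attack and MagicAttack.
; Each input event casts the controlled pawn afresh, although the construction script also stores that cast in BpCharacter, which no event reads.
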(event EventBeginPlay)

(event EventTick
  (params (DeltaSeconds :type Float%20%28single-precision%29)))

(event Input|ActionEvents|InputActionAttack
  (params (Key :type Key%20Structure :default "None"))
  ;[1 1 1] Attack
  ;;[1 1 1] Physical attack
  (:Pressed
    (bind _asbp_character_2 (Utilities|Casting|CastToBP_Character_2 (Pawn|GetControlledPawn)))
    (Default|Attack _asbp_character_2)))

(event Input|ActionEvents|InputActionMagicattack
  (params (Key :type Key%20Structure :default "None"))
  ;[1 1 1] Attack
  ;;[1 1 1] Magic attack
  (:Pressed
    (bind _asbp_character_2 (Utilities|Casting|CastToBP_Character_2 (Pawn|GetControlledPawn)))
    (Default|MagicAttack _asbp_character_2)))

(event Input|AxisEvents|InputAxisUP
  (params (AxisValue :type Float%20%28single-precision%29))
  ;[1 1 1] Movement
  (bind _asbp_character_2 (Utilities|Casting|CastToBP_Character_2 (Pawn|GetControlledPawn)))
  (Pawn|Input|AddMovementInput _asbp_character_2 (Transformation|GetActorForwardVector _asbp_character_2) AxisValue false))

(event Input|AxisEvents|InputAxisRight
  (params (AxisValue :type Float%20%28single-precision%29))
  ;[1 1 1] Movement
  (bind _asbp_character_2 (Utilities|Casting|CastToBP_Character_2 (Pawn|GetControlledPawn)))
  (Pawn|Input|AddMovementInput _asbp_character_2 (Transformation|GetActorRightVector _asbp_character_2) AxisValue false))

(event Input|AxisEvents|InputAxisLookUp
  (params (AxisValue :type Float%20%28single-precision%29))
  ;[1 1 1] Camera Movement
  (bind _asbp_character_2 (Utilities|Casting|CastToBP_Character_2 (Pawn|GetControlledPawn)))
  (Pawn|Input|AddControllerPitchInput _asbp_character_2 AxisValue))

(event Input|AxisEvents|InputAxisLookRight
  (params (AxisValue :type Float%20%28single-precision%29))
  ;[1 1 1] Camera Movement
  (bind _asbp_character_2 (Utilities|Casting|CastToBP_Character_2 (Pawn|GetControlledPawn)))
  (Pawn|Input|AddControllerYawInput _asbp_character_2 AxisValue))

(fn ConstructionScript
  (bind _asbp_character_2 (Utilities|Casting|CastToBP_Character_2 (Pawn|GetControlledPawn)))
  (Variables|Default|SetbpCharacter _asbp_character_2))