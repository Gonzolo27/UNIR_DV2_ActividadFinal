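; BP_Sword is a melee weapon actor that deals damage to nearby pawns.
; Its TryMakeDamage function runs a sphere overlap around the static mesh, ignoring the owner of the component the sword is attached to, then applies the passed damage to every pawn found.
; The event graph is empty, so the hit check depends on an external caller, and debug strings print during it.
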(event EventBeginPlay)

(event Collision|EventActorBeginOverlap
  (params (OtherActor :type Actor%20Object%20Reference)))

(event EventTick
  (params (DeltaSeconds :type Float%20%28single-precision%29)))

(fn ConstructionScript)

(fn TryMakeDamage
  (params (damage :type Float%20%28single-precision%29))
  (bind _outactors (Collision|SphereOverlapActors (Transformation|GetWorldLocation (Variables|Default|GetStaticMesh)) 1.2e+02 (Utilities|Array|MakeArray "ObjectTypeQuery3") 0 (Utilities|Array|MakeArray (Components|GetOwner (Transformation|GetAttachParent (Variables|Default|GetDefaultSceneRoot))))))
  (Development|PrintString "Overlap")
  (for _array_element _outactors
    (Game|Damage|ApplyDamage _array_element damage 0 0)
    (Development|PrintString "End apply damage function")))