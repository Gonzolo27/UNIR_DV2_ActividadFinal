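; BP_Enemy is a sword-wielding enemy character that takes damage, flinches, dies and reports its defeat to the GrassLandsManager passed in through Setup.
; On BeginPlay it spawns a socketed sword and binds its health bar widget.
; Attack chains a two-hit montage combo through next-section switching, blocked while IsRetro is set.
; Damage picks a flinch section from the attack montage state, with sections in AttackMoves skipping the flinch; MagicAttack is an empty stub.
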(event Custom|Attack
  (bind _mesh (Variables|Character|GetMesh))
  (bind _returnvalue (Components|SkeletalMesh|GetAnimInstance _mesh))
  (bind _returnvalue_2 (Animation|Montage|MontageGetCurrentSection _returnvalue 0))
  (if (not (Variables|Default|GetisRetro))
    (if (Class|AnimInstance|MontageIsActive _returnvalue "/Game/MyAssets/Enemy/Anims/AttackMontage.AttackMontage")
      (switch name _returnvalue_2
        (:Attack_1
          (Class|AnimInstance|MontageSetNextSection _returnvalue _returnvalue_2 "Attack_2" "/Game/MyAssets/Enemy/Anims/AttackMontage.AttackMontage")))
      (else
        (Animation|PlayAnimMontage "/Game/MyAssets/Enemy/Anims/AttackMontage.AttackMontage" 1.0 "Attack_1")))))

(event Custom|MagicAttack)

(event Custom|CreateSword
  (bind _returnvalue (Game|SpawnActorfromClass "/Game/MyAssets/Sword/BP_Sword.BP_Sword_C" (Transformation|GetActorTransform) "Undefined" 0 0))
  (Transformation|AttachComponentToComponent _returnvalue (Variables|Character|GetMesh) "Sword" "SnapToTarget" "SnapToTarget" "SnapToTarget" true)
  (Variables|Default|SetbpSword _returnvalue))

(event EventBeginPlay
  (CallFunction|CreateSword)
  (bind _asui_enemy_health_bar (Utilities|Casting|CastToUI_Enemy_HealthBar (UserInterface|GetUserWidgetObject (Variables|Default|GetHealthBar))))
  (Default|SetHealth _asui_enemy_health_bar self))

(event Collision|EventActorBeginOverlap
  (params (OtherActor :type Actor%20Object%20Reference)))

(event EventTick
  (params (DeltaSeconds :type Float%20%28single-precision%29)))

(event Game|Damage|EventAnyDamage
  (params (Damage :type Float%20%28single-precision%29) (DamageType :type Damage%20Type%20Object%20Reference) (InstigatedBy :type Controller%20Object%20Reference) (DamageCauser :type Actor%20Object%20Reference))
  (bind _mesh (Variables|Character|GetMesh))
  (bind _returnvalue (Components|SkeletalMesh|GetAnimInstance _mesh))
  (Development|PrintString (Utilities|String|ToString(Float) Damage))
  (bind _output_get (Variables|Default|Sethealth (- (Variables|Default|Gethealth) Damage)))
  (if (<= _output_get 0.0)
    (Utilities|FlowControl|DoOnce false
      (:Completed
        (Variables|Default|SetisRetro true)
        (Pawn|Components|CharacterMovement|DisableMovement (Variables|Character|GetCharacterMovement))
        (bind _returnvalue_2 (Animation|PlayAnimMontage "/Game/MyAssets/Enemy/Anims/DeathMontage.DeathMontage" 1.0 "None"))
        (Utilities|FlowControl|Delay _returnvalue_2)
        (Actor|DestroyActor (Variables|Default|GetbpSword))
        (Actor|DestroyActor)
        (Default|EnemyDefeated (Variables|Default|GetgrassLandsManager))))
    (else
      (Variables|Default|SetisRetro true)
      (if (Class|AnimInstance|MontageIsActive _returnvalue "/Game/MyAssets/Enemy/Anims/AttackMontage.AttackMontage")
        (if (Utilities|Array|ContainsItem (Variables|Default|GetAttackMoves) (Animation|Montage|MontageGetCurrentSection _returnvalue 0))
          (Variables|Default|SetisRetro false)
          (else
            (bind _returnvalue_3 (Animation|PlayAnimMontage "/Game/MyAssets/Enemy/Anims/FlinchMontage.FlinchMontage" 1.0 "FlinchBigSection"))
            (Utilities|FlowControl|Delay _returnvalue_3)
            (Variables|Default|SetisRetro false)))
        (else
          (bind _returnvalue_4 (Animation|PlayAnimMontage "/Game/MyAssets/Enemy/Anims/FlinchMontage.FlinchMontage" 1.0 "FlinchSmallSection"))
          (Utilities|FlowControl|Delay _returnvalue_4)
          (Variables|Default|SetisRetro false))))))

(fn ConstructionScript)

(fn Setup
  (params (grassLandsManager :type BP%20Grass%20Lands%20Manager%20Object%20Reference))
  (Variables|Default|SetgrassLandsManager grassLandsManager))