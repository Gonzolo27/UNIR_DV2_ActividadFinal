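; BP_GameManager is the game manager actor that runs the win or lose ending sequence.
; On BeginPlay it passes itself to GrassLandsManager's Setup and pre-creates the end-game widget.
; EndGame disables player input, blends the view to an end camera, and picks text and sound based on IsGameWon.
; It then shows the widget with UI-only input and a visible mouse cursor.
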(event Custom|EndGame
  (bind _returnvalue (Game|GetPlayerController 0))
  (bind _returnvalue_2 (Game|GetPlayerController 0))
  (bind _uiendgame (Variables|Default|GetuiEndGame))
  (Input|DisableInput _returnvalue 0)
  (Game|Player|SetViewTargetwithBlend _returnvalue (Variables|Default|GetendCamera) 4.0 "VTBlend_Linear" 0.0 true)
  (if (Variables|Default|GetisGameWon)
    (Variables|/Game/Blueprints/UI/UI_EndGame.UI_EndGame_C|SetEndText _uiendgame (Variables|Default|GetwinText))
    (Audio|PlaySound2D "/Game/MyAssets/Sounds/Fanfarria.Fanfarria" 1.0 1.0 0.0 0 0)
    (else
      (Variables|/Game/Blueprints/UI/UI_EndGame.UI_EndGame_C|SetEndText _uiendgame (Variables|Default|GetloseText))
      (Audio|PlaySound2D "/Game/MyAssets/Sounds/Sad.Sad" 1.0 1.0 0.0 0 0)))
  (UserInterface|Viewport|AddtoViewport _uiendgame 0)
  (Input|SetInputModeUIOnly _returnvalue_2 0 "DoNotLock")
  (Variables|/Script/Engine.PlayerController|SetbShowMouseCursor _returnvalue_2 true))

(event EventBeginPlay
  (Default|Setup (Variables|Default|GetgrassLandsManager) self)
  (bind _returnvalue (UserInterface|CreateWidget "/Game/Blueprints/UI/UI_EndGame.UI_EndGame_C"))
  (Variables|Default|SetuiEndGame _returnvalue))

(event Collision|EventActorBeginOverlap
  (params (OtherActor :type Actor%20Object%20Reference)))

(event EventTick
  (params (DeltaSeconds :type Float%20%28single-precision%29)))

(fn ConstructionScript)