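; BP_Ice_Door is a double door in the IceLands area that opens for the player once the level's trial is passed.
; When BP_Character_2 overlaps the Box trigger, it checks IceLandsManager.IsTrialPassed and calls EOpenDoor on LeftDoor and RightDoor.
; The IsDoorOpen flag makes the opening one-shot, and the Blueprint has no logic to close the doors.
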(event OnComponentBeginOverlap(Box)
  (params (OverlappedComponent :type Primitive%20Component%20Object%20Reference) (OtherActor :type Actor%20Object%20Reference) (OtherComp :type Primitive%20Component%20Object%20Reference) (OtherBodyIndex :type Integer) (bFromSweep :type Boolean) (SweepResult :type Hit%20Result%20Structure%20%28by%20ref%29))
  (if (not (Variables|Default|GetisDoorOpen))
    (Utilities|Casting|CastToBP_Character_2 OtherActor)
    (if (Variables|/Game/Blueprints/IceLands/BP_IceLandsManager.BP_IceLandsManager_C|GetisTrialPassed (Variables|Default|GeticeLandsManager))
      (Variables|Default|SetisDoorOpen true)
      (Default|EOpenDoor (Variables|Default|GetleftDoor))
      (Default|EOpenDoor (Variables|Default|GetrightDoor)))))

(event EventBeginPlay)

(event Collision|EventActorBeginOverlap
  (params (OtherActor :type Actor%20Object%20Reference)))

(event EventTick
  (params (DeltaSeconds :type Float%20%28single-precision%29)))

(fn ConstructionScript)