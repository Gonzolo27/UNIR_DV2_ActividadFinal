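; Interactable IceLands button that forms part of an ordered door puzzle coordinated by a DoorManager.
; Overlapping its box with BP_Character_2 enables player input, so the Interaction action can press it when not already pressed.
; Press and Release use timelines to slide the actor along world X and update IsPressed.
; A finished press sends IndexOrder to the DoorManager, injected through SetUp, for order checking.
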(event OnComponentBeginOverlap(Box)
  (params (OverlappedComponent :type Primitive%20Component%20Object%20Reference) (OtherActor :type Actor%20Object%20Reference) (OtherComp :type Primitive%20Component%20Object%20Reference) (OtherBodyIndex :type Integer) (bFromSweep :type Boolean) (SweepResult :type Hit%20Result%20Structure%20%28by%20ref%29))
  (Utilities|Casting|CastToBP_Character_2 OtherActor)
  (Input|EnableInput (Game|GetPlayerController 0)))

(event OnComponentEndOverlap(Box)
  (params (OverlappedComponent :type Primitive%20Component%20Object%20Reference) (OtherActor :type Actor%20Object%20Reference) (OtherComp :type Primitive%20Component%20Object%20Reference) (OtherBodyIndex :type Integer))
  (Utilities|Casting|CastToBP_Character_2 OtherActor)
  (Input|DisableInput (Game|GetPlayerController 0)))

(event Custom|Release
  ;[1 1 1] Release button
  (Variables|Default|SetstartPos (Transformation|GetActorLocation))
  (Utilities|FlowControl|Sequence
    (:then_0
      (bind _unpulse (Timeline|Timeline_2 SetNewTime)
        (:Update
          (Transformation|SetActorLocation (Math|Vector|MakeVector (+ _unpulse (.x (Variables|Default|GetstartPos))) (.y (Variables|Default|GetstartPos)) (.z (Variables|Default|GetstartPos))) false false))
        (:Finished
          (Variables|Default|SetstartPos (Transformation|GetActorLocation))
          (Variables|Default|SetisPressed false))))
    (:then_1
      (Timeline|Timeline_2 Play))))

(event Custom|Press
  ;[1 1 1] PressButton
  (Variables|Default|SetstartPos (Transformation|GetActorLocation))
  (Utilities|FlowControl|Sequence
    (:then_0
      (bind _pulse (Timeline|Timeline_1 SetNewTime)
        (:Update
          (Transformation|SetActorLocation (Math|Vector|MakeVector (+ _pulse (.x (Variables|Default|GetstartPos))) (.y (Variables|Default|GetstartPos)) (.z (Variables|Default|GetstartPos))) false false))
        (:Finished
          (Variables|Default|SetstartPos (Transformation|GetActorLocation))
          (Variables|Default|SetisPressed true)
          (Default|CheckOrder (Variables|Default|GetdoorManager) (Variables|Default|GetindexOrder)))))
    (:then_1
      (Timeline|Timeline_1 Play))))

(event EventBeginPlay)

(event EventTick
  (params (DeltaSeconds :type Float%20%28single-precision%29)))

(event Input|ActionEvents|InputActionInteraction
  (params (Key :type Key%20Structure))
  (:Pressed
    (if (not (Variables|Default|GetisPressed))
      (CallFunction|Press)
      (Development|PrintString "ButtonPressed" true true "(R=0.000000,G=0.660000,B=1.000000,A=1.000000)" 1e+01))))

(fn ConstructionScript)

(fn SetUp
  (params (doorManager :type BP%20Ice%20Lands%20Manager%20Object%20Reference))
  (Variables|Default|SetdoorManager doorManager))