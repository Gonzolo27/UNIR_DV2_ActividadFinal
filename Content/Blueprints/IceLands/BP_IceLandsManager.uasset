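; BP_IceLandsManager runs an ordered-button puzzle for the IceLands area.
; On BeginPlay it passes itself to each button through SetUp, and CheckOrder compares a given value against the expected sequence.
; A correct value advances the index or, at the end, marks the trial passed; a wrong one restarts it and releases pressed buttons.
; Door opening is still a TODO, and ResetButtons has its release logic disconnected.
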(event EventBeginPlay
  (for _array_element (Variables|Default|GetbpButtons)
    (Default|SetUp _array_element self)))

(event Collision|EventActorBeginOverlap
  (params (OtherActor :type Actor%20Object%20Reference)))

(event EventTick
  (params (DeltaSeconds :type Float%20%28single-precision%29)))

(fn ConstructionScript)

(fn CheckOrder
  (params (value :type Integer))
  ;[1 1 1] Comprueba si el valor actual del array coincide con el valor del botón pulsado
  (if (== value (Utilities|Array|Get(acopy) (Variables|Default|GetbuttonsOrder) (Variables|Default|GetactualIndex)))
    ;[1 1 1] Comprueba si ha llegado al final del array
    (if (== (+ (Variables|Default|GetactualIndex) 1) (Utilities|Array|Length (Variables|Default|GetbuttonsOrder)))
      ;[1 1 1] TODO: ha llegado al final, la puerta se abre
      (Development|PrintString "End" true true "(R=0.000000,G=0.660000,B=1.000000,A=1.000000)" 1e+01)
      (Variables|Default|SetisTrialPassed true)
      (else
        (Math|Integer|IncrementInt (Variables|Default|GetactualIndex))))
    (else
      ;[1 1 1] Reiniciar botones
      (Development|PrintString "Mal")
      (Variables|Default|SetactualIndex 0)
      (for _array_element (Variables|Default|GetbpButtons)
        (if (Variables|/Game/Blueprints/IceLands/BP_Button.BP_Button_C|GetisPressed _array_element)
          (Default|Release _array_element))))))

(fn ResetButtons
  (for _array_element (Variables|Default|GetbpButtons)
    _))