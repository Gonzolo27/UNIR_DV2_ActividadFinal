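; Ice Lands door that acts as an ordered button puzzle, checking button presses against a required sequence.
; The construction script passes the door to each linked button through SetUp.
; CheckOrder compares a value to the current ButtonsOrder entry, advancing and printing the index on a match or resetting it on a miss.
; Completing the sequence triggers nothing yet, and resetting the buttons is still a TODO.
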(event EventBeginPlay)

(event Collision|EventActorBeginOverlap
  (params (OtherActor :type Actor%20Object%20Reference)))

(event EventTick
  (params (DeltaSeconds :type Float%20%28single-precision%29)))

(fn ConstructionScript
  (for _array_element (Variables|Default|GetbpButtons)
    (Default|SetUp _array_element self)))

(fn CheckOrder
  (params (value :type Integer))
  ;[1 1 1] Comprueba si el valor actual del array coincide con el valor del botón pulsado
  (if (== value (Utilities|Array|Get(acopy) (Variables|Default|GetbuttonsOrder) (Variables|Default|GetactualIndex)))
    ;[1 1 1] Comprueba si ha llegado al final del array
    (if (not (== (+ (Variables|Default|GetactualIndex) 1) (Utilities|Array|Length (Variables|Default|GetbuttonsOrder))))
      (bind _result (Math|Integer|IncrementInt (Variables|Default|GetactualIndex))
        (:%20%20
          (Development|PrintString (Utilities|String|Append "Actual index: " (Utilities|String|ToString(Integer) _result))))))
    (else
      ;[1 1 1] TODO: Reiniciar botones (animación y pulsable - boolean -)
      (Variables|Default|SetactualIndex 0))))