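; Combat character with health, mana, a socket-attached sword, a HUD widget and montage-driven melee and magic attacks.
; Attack chains montage sections into a combo, while MagicAttack spends slowly regenerating mana and ThrowMagic spawns the projectile.
; Damage triggers small or big flinches, skipped during listed attack sections, with IsRetro blocking attacks meanwhile.
; At zero health it plays a death montage once, then removes sword, UI and itself.
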(event Custom|Attack
  (bind _mesh (Variables|Character|GetMesh))
  (bind _returnvalue (Components|SkeletalMesh|GetAnimInstance _mesh))
  (bind _returnvalue_2 (Animation|Montage|MontageGetCurrentSection _returnvalue 0))
  ;[1 1 1] Physical attack
  (if (not (Variables|Default|GetisRetro))
    (if (Class|AnimInstance|MontageIsActive _returnvalue "/Game/MyAssets/Enemy/Anims/AttackMontage.AttackMontage")
      (switch name _returnvalue_2
        (:Attack_1
          (Class|AnimInstance|MontageSetNextSection _returnvalue _returnvalue_2 (Utilities|Array|Get(acopy) (Variables|Default|GetAttackMoves) 1) "/Game/MyAssets/Enemy/Anims/AttackMontage.AttackMontage")))
      (else
        (Animation|PlayAnimMontage "/Game/MyAssets/Enemy/Anims/AttackMontage.AttackMontage" 1.0 (Utilities|Array|Get(acopy) (Variables|Default|GetAttackMoves)))))))

(event Custom|MagicAttack
  ;[1 1 1] Magic attack
  (if (and (not (Variables|Default|GetisRetro)) (>= (Variables|Default|Getmana) 7.0))
    (Variables|Default|Setmana (- (Variables|Default|Getmana) 7.0))
    (Animation|PlayAnimMontage "/Game/MyAssets/Enemy/Anims/MagicMontage.MagicMontage" 1.0 "None")))

(event Custom|CreateSword
  (bind _returnvalue (Game|SpawnActorfromClass "/Game/MyAssets/Sword/BP_Sword.BP_Sword_C" (Transformation|GetActorTransform) "Undefined" 0 0))
  (Transformation|AttachComponentToComponent _returnvalue (Variables|Character|GetMesh) "Sword" "SnapToTarget" "SnapToTarget" "SnapToTarget" true)
  (Variables|Default|SetbpSword _returnvalue))

(event Custom|ThrowMagic
  (Game|SpawnActorfromClass "/Game/Blueprints/BP_Projectil.BP_Projectil_C" (Transformation|GetWorldTransform (Variables|Default|GetArrowToProjectile)) "Undefined" 0 self))

(event Custom|RegenerateMana
  (if (< (Variables|Default|Getmana) (Variables|Default|GetmaxMana))
    (Variables|Default|Setmana (+ (Variables|Default|Getmana) 0.25))))

(event EventBeginPlay
  (CallFunction|CreateSword)
  (bind _returnvalue (UserInterface|CreateWidget "/Game/Blueprints/UI/UI_Character.UI_Character_C"))
  (bind _output_get (Variables|Default|SetUIRef _returnvalue))
  (UserInterface|Viewport|AddtoViewport _output_get 0)
  (Utilities|Time|SetTimerbyEvent (delegate Custom|RegenerateMana) 1.0 true 1.0))

(event Collision|EventActorBeginOverlap
  (params (OtherActor :type Actor%20Object%20Reference)))

(event EventTick
  (params (DeltaSeconds :type Float%20%28single-precision%29)))

(event Game|Damage|EventAnyDamage
  (params (Damage :type Float%20%28single-precision%29) (DamageType :type Damage%20Type%20Object%20Reference) (InstigatedBy :type Controller%20Object%20Reference) (DamageCauser :type Actor%20Object%20Reference))
  (bind _mesh (Variables|Character|GetMesh))
  (bind _returnvalue (Components|SkeletalMesh|GetAnimInstance _mesh))
  (bind _output_get (Variables|Default|Sethealth (- (Variables|Default|Gethealth) Damage)))
  (if (<= _output_get 0.0)
    (Utilities|FlowControl|DoOnce false
      (:Completed
        (Variables|Default|SetisRetro true)
        (Pawn|Components|CharacterMovement|DisableMovement (Variables|Character|GetCharacterMovement))
        (bind _returnvalue_2 (Animation|PlayAnimMontage "/Game/MyAssets/Enemy/Anims/DeathMontage.DeathMontage" 1.0 "None"))
        (Utilities|FlowControl|Delay _returnvalue_2)
        (Actor|DestroyActor (Variables|Default|GetbpSword))
        (Widget|RemovefromParent (Variables|Default|GetUIRef))
        (Actor|DestroyActor)))
    (else
      (Variables|Default|SetisRetro true)
      (if (Class|AnimInstance|MontageIsActive _returnvalue "/Game/MyAssets/Enemy/Anims/AttackMontage.AttackMontage")
        (if (Utilities|Array|ContainsItem (Variables|Default|GetAttackMoves) (Animation|Montage|MontageGetCurrentSection _returnvalue 0))
          (Variables|Default|SetisRetro false)
          (else
            (bind _returnvalue_3 (Animation|PlayAnimMontage "/Game/MyAssets/Enemy/Anims/FlinchMontage.FlinchMontage" 1.0 "FlinchBigSection"))
            (Utilities|FlowControl|Delay _returnvalue_3)
            (Variables|Default|SetisRetro false)))
        (else
          (bind _returnvalue_4 (Animation|PlayAnimMontage "/Game/MyAssets/Enemy/Anims/FlinchMontage.FlinchMontage" 1.0 "FlinchSmallSection"))
          (Utilities|FlowControl|Delay _returnvalue_4)
          (Variables|Default|SetisRetro false))))))

(fn ConstructionScript)