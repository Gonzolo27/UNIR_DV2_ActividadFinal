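; BP_Statue is a moving statue obstacle in AsianLands that has the manager reset the player's position when it hits BP_Character_2.
; At BeginPlay, StatueType selects one of three speed timelines that offset the statue from its start location, along X for Slow and Medium, Y for Fast.
; IsReverse flips the offset direction, and Setup supplies the AsianLandsManager reference used on hit.
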(event OnComponentHit(StaticMeshComponent)
  (params (HitComponent :type Primitive%20Component%20Object%20Reference) (OtherActor :type Actor%20Object%20Reference) (OtherComp :type Primitive%20Component%20Object%20Reference) (NormalImpulse :type Vector :default "0, 0, 0") (Hit :type Hit%20Result%20Structure%20%28by%20ref%29))
  (Utilities|Casting|CastToBP_Character_2 OtherActor)
  (Default|RestartPlayerPos (Variables|Default|GetasianLandsManager)))

(event Custom|DoTL_Slow
  (bind _goback (Timeline|TL_GoBackIn10 Play)
    (:Update
      (Variables|Default|SetnewLocation (Math|Vector|MakeVector _goback 0.0 0.0))
      (CallFunction|ChangeActorLocation (Variables|Default|GetnewLocation)))))

(event Custom|DoTL_Medium
  (bind _goback (Timeline|TL_GoBackIn8 Play)
    (:Update
      (Variables|Default|SetnewLocation (Math|Vector|MakeVector _goback 0.0 0.0))
      (CallFunction|ChangeActorLocation (Variables|Default|GetnewLocation)))))

(event Custom|DoTL_Fast
  (bind _goback (Timeline|TL_GoBackIn5 Play)
    (:Update
      (Variables|Default|SetnewLocation (Math|Vector|MakeVector 0.0 _goback 0.0))
      (CallFunction|ChangeActorLocation (Variables|Default|GetnewLocation)))))

(event EventBeginPlay
  (Variables|Default|SetstartLocation (Transformation|GetActorLocation))
  (switch Utilities|FlowControl|Switch|SwitchonstatueType (Variables|Default|GetstatueType)
    (:NewEnumerator0
      (CallFunction|DoTLSlow))
    (:NewEnumerator1
      (CallFunction|DoTLMedium))
    (:NewEnumerator2
      (CallFunction|DoTLFast))))

(event EventTick
  (params (DeltaSeconds :type Float%20%28single-precision%29)))

(fn ConstructionScript)

(fn ChangeActorLocation
  (params (NewParam :type Vector))
  (bind _startlocation (Variables|Default|GetstartLocation))
  (if (Variables|Default|GetisReverse)
    (Transformation|SetActorLocation (- _startlocation NewParam) false false)
    (else
      (Transformation|SetActorLocation (+ _startlocation NewParam) false false))))

(fn Setup
  (params (asianLandsManager :type BP%20Asian%20Lands%20Manager%20Object%20Reference))
  (Variables|Default|SetasianLandsManager asianLandsManager))