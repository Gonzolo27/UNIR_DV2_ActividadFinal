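; HealthSpawner is a spawner actor that places ItemHealth pickups at its SpawnPoint in the level.
; On BeginPlay it spawns an item immediately and passes itself to that item through Setup.
; Its GenerateItem event waits on a fixed delay, then spawns and sets up another item the same way.
; Nothing in this graph calls GenerateItem, so respawning depends on an outside caller.
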(event Custom|GenerateItem
  (Utilities|FlowControl|Delay 1e+01)
  (bind _returnvalue (Game|SpawnActorfromClass "/Game/Blueprints/GrassLands/ItemHealth.ItemHealth_C" (Transformation|GetActorTransform (Variables|Default|GetspawnPoint)) "Undefined" 0 0))
  (Default|Setup _returnvalue self))

(event EventBeginPlay
  (bind _returnvalue (Game|SpawnActorfromClass "/Game/Blueprints/GrassLands/ItemHealth.ItemHealth_C" (Transformation|GetActorTransform (Variables|Default|GetspawnPoint)) "Undefined" 0 0))
  (Default|Setup _returnvalue self))

(event Collision|EventActorBeginOverlap
  (params (OtherActor :type Actor%20Object%20Reference)))

(event EventTick
  (params (DeltaSeconds :type Float%20%28single-precision%29)))

(fn ConstructionScript)