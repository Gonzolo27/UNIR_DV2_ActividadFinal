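; BP_GrassLandsManager tracks enemy defeats in the GrassLands area and detects when all spawned enemies are beaten.
; On BeginPlay it passes itself to its EnemySpawner through Setup.
; Each EnemyDefeated event increments a counter and compares it to the spawner's MaxEnemiesToSpawn.
; Reaching that limit only prints an on-screen finish message, with no further completion logic.
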(event Custom|EnemyDefeated
  (bind _result (Math|Integer|IncrementInt (Variables|Default|GetenemeisDefeated))
    (:%20%20
      (if (>= _result (Variables|/Game/Blueprints/EnemySpawner.EnemySpawner_C|GetmaxEnemiesToSpawn (Variables|Default|GetenemySpawner)))
        (Development|PrintString "FINISH!!!!!!!!!!" true true "(R=0.000000,G=0.660000,B=1.000000,A=1.000000)" 3e+01)))))

(event EventBeginPlay
  (Default|Setup (Variables|Default|GetenemySpawner) self))

(event Collision|EventActorBeginOverlap
  (params (OtherActor :type Actor%20Object%20Reference)))

(event EventTick
  (params (DeltaSeconds :type Float%20%28single-precision%29)))

(fn ConstructionScript)