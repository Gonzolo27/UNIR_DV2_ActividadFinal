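; Grasslands enemy spawner that starts a one-shot wave when BP_Character_2 overlaps it.
; A looping timer, optionally preceded by an immediate spawn, creates BP_Enemy at random SpawnPoints until MaxEnemiesToSpawn is reached, then pauses.
; Each enemy receives the GrassLandsManager passed through Setup, and each spawn plays a bounce notification widget.
; Location and rotation use separate random rolls, so they can come from different spawn points.
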(event Custom|ESpawnEnemy
  (CallFunction|SpawnEnemy)
  (CallFunction|PlayUiNotifySpawnEnemy)
  (if (>= (Variables|Default|GetactualEnemiesSpawned) (Variables|Default|GetmaxEnemiesToSpawn))
    (Utilities|Time|PauseTimerbyHandle (stale Collision|EventActorBeginOverlap _returnvalue))))

(event Custom|playUiNotifySpawnEnemy
  (bind _uinotifspawnenemy (Variables|Default|GetuiNotifSpawnEnemy))
  (UserInterface|Animation|PlayAnimation _uinotifspawnenemy (Variables|/Game/Blueprints/UI/UI_NotificationEnemySpawn.UI_NotificationEnemySpawn_C|GetBounce _uinotifspawnenemy) 0.0 1 "Forward" 1.0 false))

(event EventBeginPlay
  (bind _returnvalue (UserInterface|CreateWidget "/Game/Blueprints/UI/UI_NotificationEnemySpawn.UI_NotificationEnemySpawn_C"))
  (bind _output_get (Variables|Default|SetuiNotifSpawnEnemy _returnvalue))
  (UserInterface|Viewport|AddtoViewport _output_get 0))

(event Collision|EventActorBeginOverlap
  (params (OtherActor :type Actor%20Object%20Reference))
  (if (Variables|Default|GetcanSpawnEnemies)
    (Development|PrintString (Utilities|String|Append "actualEnemiesSpawned: " (Utilities|String|ToString(Integer) (Variables|Default|GetactualEnemiesSpawned))))
    (Utilities|Casting|CastToBP_Character_2 OtherActor)
    (Variables|Default|SetcanSpawnEnemies false)
    (if (Variables|Default|GetspawnFirstWithoutWait)
      (CallFunction|PlayUiNotifySpawnEnemy)
      (CallFunction|SpawnEnemy)
      (if (not (>= (Variables|Default|GetactualEnemiesSpawned) (Variables|Default|GetmaxEnemiesToSpawn)))
        (bind _returnvalue (Utilities|Time|SetTimerbyEvent (delegate Custom|ESpawnEnemy) (Variables|Default|GettimeBetweenSpawn) true :!label _label)))
      (else
        (goto _label)))))

(event EventTick
  (params (DeltaSeconds :type Float%20%28single-precision%29)))

(fn ConstructionScript)

(fn SpawnEnemy
  (bind _spawnpoints (Variables|Default|GetspawnPoints))
  (bind _returnvalue (Utilities|Array|Length _spawnpoints))
  (bind _returnvalue_2 (- _returnvalue 1))
  (bind _returnvalue_3 (Math|Random|RandomIntegerinRange 0 _returnvalue_2))
  (bind _output (Utilities|Array|Get(acopy) _spawnpoints _returnvalue_3))
  (bind _returnvalue_4 (Transformation|GetActorTransform _output))
  (Development|PrintString (Utilities|String|Append "SpawnPoints length: " (Utilities|String|ToString(Integer) _returnvalue) " / random number: " (Utilities|String|ToString(Integer) _returnvalue_3)))
  (bind _returnvalue_5 (AI|SpawnAIFromClass "/Game/Blueprints/Characters/Enemy/BP_Enemy.BP_Enemy_C" 0 (.location _returnvalue_4) (.rotation _returnvalue_4) false 0))
  (bind _asbp_enemy (Utilities|Casting|CastToBP_Enemy _returnvalue_5))
  (Default|Setup _asbp_enemy (Variables|Default|GetgrassLandsManager))
  (Math|Integer|IncrementInt (Variables|Default|GetactualEnemiesSpawned)
    (:%20%20
      (Development|PrintString "Spawning enemy" true true "(R=1.000000,G=0.000000,B=0.098436,A=1.000000)"))))

(fn Setup
  (params (grassLandsManager :type BP%20Grass%20Lands%20Manager%20Object%20Reference))
  (Variables|Default|SetgrassLandsManager grassLandsManager))