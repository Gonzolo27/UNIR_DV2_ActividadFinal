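; BP_FireMovableDoor is a door actor in the FireLands content that moves vertically when opened.
; Its EOpenDoor event runs only if CanBeOpen is set and the door is not already open, then caches the start position and sets IsDoorOpen.
; The OpenDoor timeline adds its OpenDoorUp track value to the starting Z on each update, with no closing logic.
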(event Custom|EOpenDoor
  (if (and (not (Variables|Default|GetisDoorOpen)) (Variables|Default|GetcanBeOpen))
    (Variables|Default|SetstartPos (Transformation|GetActorLocation))
    (Variables|Default|SetisDoorOpen true)
    (bind _opendoorup (Timeline|openDoor Play)
      (:Update
        (Transformation|SetActorLocation (Math|Vector|MakeVector (.x (Variables|Default|GetstartPos)) (.y (Variables|Default|GetstartPos)) (+ _opendoorup (.z (Variables|Default|GetstartPos)))) false false)))))

(event EventBeginPlay)

(event Collision|EventActorBeginOverlap
  (params (OtherActor :type Actor%20Object%20Reference)))

(event EventTick
  (params (DeltaSeconds :type Float%20%28single-precision%29)))

(fn ConstructionScript)