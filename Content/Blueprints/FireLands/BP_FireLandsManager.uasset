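; BP_FireLandsManager is the manager actor for the FireLands area, linking its doors and end point.
; On BeginPlay it passes itself to FireDoor and EndPoint through their setup calls.
; It exposes events that forward to FireMovableDoor, one setting it as openable and the other calling its open event.
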(event Custom|EOpenDoor
  (Default|EOpenDoor (Variables|Default|GetfireMovableDoor)))

(event Custom|ESetOpenable
  (Variables|/Game/Blueprints/FireLands/BP_FireMovableDoor.BP_FireMovableDoor_C|SetcanBeOpen (Variables|Default|GetfireMovableDoor) true))

(event EventBeginPlay
  (bind _self self)
  (Default|SetUp (Variables|Default|GetfireDoor) _self)
  (Default|Setup (Variables|Default|GetendPoint) _self))

(event Collision|EventActorBeginOverlap
  (params (OtherActor :type Actor%20Object%20Reference)))

(event EventTick
  (params (DeltaSeconds :type Float%20%28single-precision%29)))

(fn ConstructionScript)